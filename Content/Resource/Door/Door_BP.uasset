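; Colored door actor that takes a Red, Yellow or Blue identity from its Color variable.
; On BeginPlay it applies the matching color material to its static mesh.
; It then writes the world position of its FinalLocation component into that color's door location variable on the GameData game instance.
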(event EventBeginPlay
  (bind _final_location (Variables|Default|GetFinal%20Location))
  (bind _returnvalue (Transformation|GetWorldLocation _final_location))
  ;[1 1 1] Set Material Color
  (Rendering|Material|SetMaterial (Variables|Default|GetStaticMesh) 0 (Utilities|Select :Index (Variables|Default|GetColor) :NewEnumerator0 "/Game/FirstPersonBP/Blueprints/Mesh/Colors_Mat_Red.Colors_Mat_Red" :NewEnumerator1 "/Game/FirstPersonBP/Blueprints/Mesh/Colors_Mat_Yellow.Colors_Mat_Yellow" :NewEnumerator2 "/Game/FirstPersonBP/Blueprints/Mesh/Colors_Mat_blue.Colors_Mat_blue"))
  ;[1 1 1] Set Gmaedata Door Location
  (bind _asgame_data (Utilities|Casting|CastToGameData (Game|GetGameInstance)))
  (switch Utilities|FlowControl|Switch|SwitchonColor_Enum (Variables|Default|GetColor)
    (:NewEnumerator0
      (Variables|/Game/Resource/GameData.GameData_C|SetDoorLoc_Red _asgame_data _returnvalue))
    (:NewEnumerator1
      (Variables|/Game/Resource/GameData.GameData_C|SetDoorLoc_Yellow _asgame_data _returnvalue))
    (:NewEnumerator2
      (Variables|/Game/Resource/GameData.GameData_C|SetDoorLoc_Blue _asgame_data _returnvalue))))

(fn ConstructionScript)