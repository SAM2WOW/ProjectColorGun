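; Human NPC that gets a random occupation, costume and starting color, then walks to the door matching its current color.
; Paint projectile hits recolor it, play a pop, check the color against its occupation's and redirect it via AIMoveTo.
; Right-colored arrivals add money and an entered count in GameData.
; Others lose money, speed up toward the exit, then count as left and lose money again.
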(event OnComponentBeginOverlap(HitBox)
  (params (OverlappedComponent :type Primitive%20Component%20Object%20Reference) (OtherActor :type Actor%20Object%20Reference) (OtherComp :type Primitive%20Component%20Object%20Reference) (OtherBodyIndex :type Integer) (bFromSweep :type Boolean) (SweepResult :type Hit%20Result%20Structure%20%28by%20ref%29))
  ;[1 1 1] Detect RIght Color
  (bind _asfirst_person_projectile (Utilities|Casting|CastToFirstPersonProjectile OtherActor))
  ;;[1 1 1] Change Material
  (Rendering|Material|SetMaterial (Variables|Character|GetMesh) 0 (Utilities|Select :Index (Variables|/Game/FirstPersonBP/Blueprints/FirstPersonProjectile.FirstPersonProjectile_C|GetBallColor _asfirst_person_projectile) :NewEnumerator0 "/Game/FirstPersonBP/Blueprints/Mesh/Colors_Mat_Red.Colors_Mat_Red" :NewEnumerator1 "/Game/FirstPersonBP/Blueprints/Mesh/Colors_Mat_Yellow.Colors_Mat_Yellow" :NewEnumerator2 "/Game/FirstPersonBP/Blueprints/Mesh/Colors_Mat_blue.Colors_Mat_blue"))
  (Variables|Default|SetCurrent%20Color (Variables|/Game/FirstPersonBP/Blueprints/FirstPersonProjectile.FirstPersonProjectile_C|GetBallColor _asfirst_person_projectile))
  (Audio|SpawnSoundatLocation "/Game/Resource/SoundFX/Pop_Sound.Pop_Sound" (Transformation|GetActorLocation) "0, 0, 0" 0.7 1.0 0.0 "/Game/Resource/SoundFX/NewSoundAttenuation.NewSoundAttenuation" 0)
  (if (== (Variables|/Game/FirstPersonBP/Blueprints/FirstPersonProjectile.FirstPersonProjectile_C|GetBallColor _asfirst_person_projectile) (Variables|Default|GetRight%20Color))
    (Variables|Default|SetRight%20Color? true)
    (else
      (Variables|Default|SetRight%20Color? false)))
  (CallFunction|Walking))

(event Custom|Walking
  ;[1 1 1] Walking
  (bind _asgame_data (Utilities|Casting|CastToGameData (Game|GetGameInstance)))
  (AI|AIMoveTo self (Utilities|Select :Index (Variables|Default|GetCurrent%20Color) :NewEnumerator0 (Variables|/Game/Resource/GameData.GameData_C|GetDoorLoc_Red _asgame_data) :NewEnumerator1 (Variables|/Game/Resource/GameData.GameData_C|GetDoorLoc_Yellow _asgame_data) :NewEnumerator2 (Variables|/Game/Resource/GameData.GameData_C|GetDoorLoc_Blue _asgame_data)) 0 2e+01 false
    (:OnSuccess
      (if (Variables|Default|GetRight%20Color?)
        (Actor|DestroyActor)
        (Audio|SpawnSoundatLocation "/Game/Resource/SoundFX/Scores_Up.Scores_Up" (Transformation|GetActorLocation) "0, 0, 0" 1.0 1.0 0.0 "/Game/Resource/SoundFX/NewSoundAttenuation.NewSoundAttenuation" 0)
        ;[1 1 1] Add Human Entered Number
        (bind _asgame_data_2 (Utilities|Casting|CastToGameData (Game|GetGameInstance)))
        (Variables|/Game/Resource/GameData.GameData_C|SetHuman%20Entered _asgame_data_2 (+ (Variables|/Game/Resource/GameData.GameData_C|GetHuman%20Entered _asgame_data_2) 1))
        ;[1 1 1] Add Money
        (Variables|/Game/Resource/GameData.GameData_C|SetMoney _asgame_data_2 (+ (Variables|/Game/Resource/GameData.GameData_C|GetMoney _asgame_data_2) 4e+02))
        (else
          (CallFunction|Leaving)
          ;[1 1 1] Subtract Money
          (bind _asgame_data_3 (Utilities|Casting|CastToGameData (Game|GetGameInstance)))
          (Variables|/Game/Resource/GameData.GameData_C|SetMoney _asgame_data_3 (- (Variables|/Game/Resource/GameData.GameData_C|GetMoney _asgame_data_3) 2e+02)))))
    (:OnFail
      (CallFunction|Leaving))))

(event Custom|Leaving
  (bind _charactermovement (Variables|Character|GetCharacterMovement))
  ;[1 1 1] Speed Up Leaving
  (Variables|/Script/Engine.CharacterMovementComponent|SetMaxWalkSpeed _charactermovement (+ (Variables|/Script/Engine.CharacterMovementComponent|GetMaxWalkSpeed _charactermovement) 3e+01))
  ;[1 1 1] Goto Exit Door
  (bind _asgame_data (Utilities|Casting|CastToGameData (Game|GetGameInstance)))
  (AI|AIMoveTo self (Variables|/Game/Resource/GameData.GameData_C|GetExit_Loc _asgame_data) 0 2e+01 false
    (:OnSuccess
      (Actor|DestroyActor)
      ;[1 1 1] Add Human Left Number
      (bind _asgame_data_2 (Utilities|Casting|CastToGameData (Game|GetGameInstance)))
      (Variables|/Game/Resource/GameData.GameData_C|SetHuman%20Left _asgame_data_2 (+ (Variables|/Game/Resource/GameData.GameData_C|GetHuman%20Left _asgame_data_2) 1))
      ;[1 1 1] Subtract Money
      (bind _asgame_data_3 (Utilities|Casting|CastToGameData (Game|GetGameInstance)))
      (Variables|/Game/Resource/GameData.GameData_C|SetMoney _asgame_data_3 (- (Variables|/Game/Resource/GameData.GameData_C|GetMoney _asgame_data_3) 2e+02)))
    (:OnFail
      (CallFunction|Leaving))))

(event EventBeginPlay
  ;[1 1 1] Random Occupation
  (bind _asgame_data (Utilities|Casting|CastToGameData (Game|GetGameInstance)))
  (bind _output_get (Variables|Default|SetIndex (Math|Random|RandomInteger (Utilities|Array|Length (Variables|/Game/Resource/GameData.GameData_C|GetOccupations _asgame_data)))))
  (Variables|Default|SetOccupation (.job (Utilities|Array|Get(acopy) (Variables|/Game/Resource/GameData.GameData_C|GetOccupations _asgame_data) _output_get)))
  (Class|SkinnedMeshComponent|SetSkeletalMesh (Variables|Default|GetCostume) (.mesh (Utilities|Array|Get(acopy) (Variables|/Game/Resource/GameData.GameData_C|GetOccupations _asgame_data) _output_get)) true)
  (Variables|Default|SetRight%20Color (.color (Utilities|Array|Get(acopy) (Variables|/Game/Resource/GameData.GameData_C|GetOccupations _asgame_data) _output_get)))
  ;[1 1 1] Random Current Color
  (Variables|Default|SetCurrent%20Color (Utilities|Enum|ByteToEnumColor_Enum (Math|Conversions|ToByte(Integer) (Math|Random|RandomInteger 3))))
  ;[1 1 1] First Walk
  (CallFunction|Walking))

(fn ConstructionScript)